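; Melee player unit pawn for the turn-based tile toolkit, extending a parent unit with skeletal mesh animation.
; Tick calls MoveAnimation on the mesh's Pawn_Anim_BP_Parent instance every frame while not idle, and a DoOnce limits it to one call upon becoming idle.
; AttackVictim and DestroyUnit run parent logic, then trigger the attack and death animations on that anim instance.
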(event `self.ReceiveTick`
  (params (DeltaSeconds :type "Float (single-precision)"))
  (`parent.ReceiveTick` DeltaSeconds)
  (if (`self.Idle`)
    (`/Engine/EditorBlueprintResources/StandardMacros.DoOnce` true :!label _label
      (:`Completed`
        _))
    (else
      (`|ExecutionSequence`
        (:`then_0`
          (goto _label :!via `Reset`))
        (:`then_1`
          _))))
  (bind _aspawn_anim_bp_parent (cast `/Game/AdvancedTurnBasedTileToolkit/Animations/Pawn_Anim_BP_Parent` (`SkeletalMeshComponent.GetAnimInstance` (`self.SkeletalMesh1`))))
  (`/Game/AdvancedTurnBasedTileToolkit/Animations/Pawn_Anim_BP_Parent.MoveAnimation` _aspawn_anim_bp_parent))

(event `self.Attack Victim`
  (params (Victim :type "/Game/AdvancedTurnBasedTileToolkit/Blueprints/Pawns/Unit_Parent Object Reference"))
  (`parent.Attack Victim` Victim)
  (bind _aspawn_anim_bp_parent (cast `/Game/AdvancedTurnBasedTileToolkit/Animations/Pawn_Anim_BP_Parent` (`SkeletalMeshComponent.GetAnimInstance` (`self.SkeletalMesh1`))))
  (`/Game/AdvancedTurnBasedTileToolkit/Animations/Pawn_Anim_BP_Parent.AttackAnimation` _aspawn_anim_bp_parent))

(event `self.Destroy Unit`
  (params (`Anim Delay` :type "Float (single-precision)"))
  (`parent.Destroy Unit` `Anim Delay`)
  (bind _aspawn_anim_bp_parent (cast `/Game/AdvancedTurnBasedTileToolkit/Animations/Pawn_Anim_BP_Parent` (`SkeletalMeshComponent.GetAnimInstance` (`self.SkeletalMesh1`))))
  (`/Game/AdvancedTurnBasedTileToolkit/Animations/Pawn_Anim_BP_Parent.DeathAnimation` _aspawn_anim_bp_parent))

(fn `UserConstructionScript`
  (`parent.UserConstructionScript`))